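; Bullet projectile actor that destroys any EnemyCharacter it hits.
; On BeginPlay it launches its static mesh with a physics impulse along the root's forward vector, scaled by Force.
; Any hit sets the mesh to ignore the Pawn channel, and the bullet itself persists.
; A Tick-accumulated timer destroys the bullet after about three seconds.
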(event `self.ReceiveBeginPlay`
  (`PrimitiveComponent.AddImpulse` (`self.StaticMesh`) (* (`SceneComponent.GetForwardVector` (`self.DefaultSceneRoot`)) (`self.Force`)) "None" false))

(event `self.ReceiveTick`
  (params (DeltaSeconds :type "Float (single-precision)"))
  (bind _output_get (set `self.Timer` (+ (`self.Timer`) DeltaSeconds)))
  (`/Engine/EditorBlueprintResources/StandardMacros.CompareFloat` _output_get 3.0
    (:`>`
      (`self.K2_DestroyActor`))))

(event `self.ReceiveHit`
  (params (MyComp :type "PrimitiveComponent Object Reference") (Other :type "Actor Object Reference") (OtherComp :type "PrimitiveComponent Object Reference") (bSelfMoved :type Boolean) (HitLocation :type "Vector Structure") (HitNormal :type "Vector Structure") (NormalImpulse :type "Vector Structure") (Hit :type "HitResult Structure (by ref)"))
  (`PrimitiveComponent.SetCollisionResponseToChannel` (`self.StaticMesh`) "ECC_Pawn" "ECR_Ignore")
  (bind _asenemy_character (cast `/Game/Custom_BPs/EnemyCharacter` Other))
  (`self.K2_DestroyActor` _asenemy_character))

(fn `UserConstructionScript`)